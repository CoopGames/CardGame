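; Game mode for a two-player, single-screen card game, driving the UI flow from name entry through deck selection and loading screen to the board.
; Stores both players' names and cards, enabling start once both have 30-card decks.
; Highlights free board slots by card type and the current round's side, and relays the pending spell card's effect values.
; Saves decks and deck-name lists through DeckSpeicher SaveGame slots.
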(event `self.ReceiveBeginPlay`
  (bind _returnvalue (`GameplayStatics.GetPlayerController` 0))
  (bind _existiert_ (`self.ÜberprüfeSpeicherstand`))
  (if _existiert_
    (`self.LadeSpeicher` "")
    (else
      (`self.Speichern` "")))
  (bind _returnvalue_2 (`|CreateWidget` "/Game/Game/UI/Game/1VS1/1VS1NameSetzen.1VS1NameSetzen_C" _returnvalue))
  (bind _output_get (set `self.NameSetzenWBPRef` _returnvalue_2))
  (`UserWidget.AddToViewport` _output_get 0)
  (`WidgetBlueprintLibrary.SetInputMode_UIOnlyEx` _returnvalue)
  (set `PlayerController.bShowMouseCursor` true _returnvalue))

(event `SetzeName`
  (params (Spieler1 :type String) (Spieler2 :type String))
  (set `self.Name1` Spieler1)
  (set `self.Name2` Spieler2))

(event `SetzeGewählteKarten`
  (params (Spieler1 :type "Array of Integer"))
  (set `self.Spieler1Karten` Spieler1)
  (set `self.Spieler1Bereit` true)
  (`self.AlleBereit`))

(event `SetzeGewählteKarten2`
  (params (`Spieler 2` :type "Array of Integer"))
  (set `self.Spieler2Karten` `Spieler 2`)
  (set `self.Spieler2Bereit` true)
  (`self.AlleBereit`))

(event `DeckSetzErstellen`
  (bind _returnvalue (`|CreateWidget` "/Game/Game/UI/Game/1VS1/Deckwählen.Deckwählen_C" (`GameplayStatics.GetPlayerController` 0)))
  (bind _output_get (set `self.DeckRef` _returnvalue))
  (`UserWidget.AddToViewport` _output_get 0))

(event `SpielStarten`
  (if (`self.Bereit`)
    (`Widget.RemoveFromParent` (`self.DeckRef`))
    (bind _returnvalue (`|CreateWidget` "/Game/Game/UI/Game/1VS1/1VS1LoadingScreen.1VS1LoadingScreen_C" (`GameplayStatics.GetPlayerController` 0)))
    (bind _output_get (set `self.1VS1LoadingScreenRef` _returnvalue))
    (`UserWidget.AddToViewport` _output_get 0)))

(event `ErzeugeSpielfeld`
  (bind _returnvalue (`|CreateWidget` "/Game/AktuelleTestregion(1VS1)/UIs/1vs1Spielfeld.1vs1Spielfeld_C" (`GameplayStatics.GetPlayerController` 0)))
  (bind _output_get (set `self.1VS1Spielfeld` _returnvalue))
  (`UserWidget.AddToViewport` _output_get 0))

(event `Spieler1KarteHinzufügenAnzeige`
  (params (ArrayLength :type Integer))
  (bind _deckref (`self.DeckRef`))
  (`/Game/Game/UI/Game/1VS1/Deckwählen.AnzahlSetzen` _deckref (`KismetStringLibrary.Conv_IntToString` ArrayLength) (`/Game/Game/UI/Game/1VS1/Deckwählen.Anzahl2` _deckref)))

(event `Spieler2KarteHinzufügenAnzeige`
  (params (ArrayLenght :type Integer))
  (bind _deckref (`self.DeckRef`))
  (`/Game/Game/UI/Game/1VS1/Deckwählen.AnzahlSetzen` _deckref (`/Game/Game/UI/Game/1VS1/Deckwählen.Anzahl1` _deckref) (`KismetStringLibrary.Conv_IntToString` ArrayLenght)))

(event `SetzeZauberKarte`
  (params (Kartenfeld :type "/Game/AktuelleTestregion(1VS1)/UIs/KartenFeld Object Reference"))
  (set `self.AktuelleZauberKarteDieAufAuswahlWartet` Kartenfeld))

(event `KartenfelderAufleuchten`
  (params (Kartentyp :type Integer) (EffektNUmmer :type Integer))
  (bind _returnvalue (== EffektNUmmer 1))
  (bind _1vs1spielfeld (`self.1VS1Spielfeld`))
  (if (`/Game/AktuelleTestregion(1VS1)/UIs/1vs1Spielfeld.Round?` _1vs1spielfeld)
    (if (== Kartentyp 0)
      (if (not _returnvalue)
        (for _array_element (`/Game/AktuelleTestregion(1VS1)/UIs/1vs1Spielfeld.PlayerBoxes` _1vs1spielfeld)
          (if (not (`/Game/AktuelleTestregion(1VS1)/UIs/KartenFeld.IsBelegt?` _array_element))
            (set `/Game/AktuelleTestregion(1VS1)/UIs/KartenFeld.CardPicture` "/Game/AktuelleTestregion(1VS1)/ImageFiles/Weiß.Weiß" _array_element))))
      (for _array_element_2 (`/Game/AktuelleTestregion(1VS1)/UIs/1vs1Spielfeld.PlayerFrontBoxes` _1vs1spielfeld)
        (if (not (`/Game/AktuelleTestregion(1VS1)/UIs/KartenFeld.IsBelegt?` _array_element_2))
          (set `/Game/AktuelleTestregion(1VS1)/UIs/KartenFeld.CardPicture` "/Game/AktuelleTestregion(1VS1)/ImageFiles/Weiß.Weiß" _array_element_2)))
      (elif (== Kartentyp 1)
        (for _array_element_3 (`/Game/AktuelleTestregion(1VS1)/UIs/1vs1Spielfeld.PlayersBuildingBoxes` _1vs1spielfeld)
          (if (not (`/Game/AktuelleTestregion(1VS1)/UIs/KartenFeld.IsBelegt?` _array_element_3))
            (set `/Game/AktuelleTestregion(1VS1)/UIs/KartenFeld.CardPicture` "/Game/AktuelleTestregion(1VS1)/ImageFiles/Weiß.Weiß" _array_element_3)))
        (elif (== Kartentyp 2)
          (for _array_element_4 (`/Game/AktuelleTestregion(1VS1)/UIs/1vs1Spielfeld.PlayerZauberplätze` _1vs1spielfeld)
            (if (not (`/Game/AktuelleTestregion(1VS1)/UIs/KartenFeld.IsBelegt?` _array_element_4))
              (set `/Game/AktuelleTestregion(1VS1)/UIs/KartenFeld.CardPicture` "/Game/AktuelleTestregion(1VS1)/ImageFiles/Weiß.Weiß" _array_element_4))))))
    (elif (== Kartentyp 0)
      (if (not _returnvalue)
        (for _array_element_5 (`/Game/AktuelleTestregion(1VS1)/UIs/1vs1Spielfeld.EnemyBoxes` _1vs1spielfeld)
          (if (not (`/Game/AktuelleTestregion(1VS1)/UIs/KartenFeld.IsBelegt?` _array_element_5))
            (set `/Game/AktuelleTestregion(1VS1)/UIs/KartenFeld.CardPicture` "/Game/AktuelleTestregion(1VS1)/ImageFiles/Weiß.Weiß" _array_element_5))))
      (for _array_element_6 (`/Game/AktuelleTestregion(1VS1)/UIs/1vs1Spielfeld.EnemyFrontBoxes` _1vs1spielfeld)
        (if (not (`/Game/AktuelleTestregion(1VS1)/UIs/KartenFeld.IsBelegt?` _array_element_6))
          (set `/Game/AktuelleTestregion(1VS1)/UIs/KartenFeld.CardPicture` "/Game/AktuelleTestregion(1VS1)/ImageFiles/Weiß.Weiß" _array_element_6)))
      (elif (== Kartentyp 1)
        (for _array_element_7 (`/Game/AktuelleTestregion(1VS1)/UIs/1vs1Spielfeld.EnemyBuildingsBoxes` _1vs1spielfeld)
          (if (not (`/Game/AktuelleTestregion(1VS1)/UIs/KartenFeld.IsBelegt?` _array_element_7))
            (set `/Game/AktuelleTestregion(1VS1)/UIs/KartenFeld.CardPicture` "/Game/AktuelleTestregion(1VS1)/ImageFiles/Weiß.Weiß" _array_element_7)))
        (elif (== Kartentyp 2)
          (for _array_element_8 (`/Game/AktuelleTestregion(1VS1)/UIs/1vs1Spielfeld.EnemyZauberplätze` _1vs1spielfeld)
            (if (not (`/Game/AktuelleTestregion(1VS1)/UIs/KartenFeld.IsBelegt?` _array_element_8))
              (set `/Game/AktuelleTestregion(1VS1)/UIs/KartenFeld.CardPicture` "/Game/AktuelleTestregion(1VS1)/ImageFiles/Weiß.Weiß" _array_element_8))))))))

(event `KartenfelderAbleuchten`
  (bind _1vs1spielfeld (`self.1VS1Spielfeld`))
  (if (`/Game/AktuelleTestregion(1VS1)/UIs/1vs1Spielfeld.Round?` _1vs1spielfeld)
    (for _array_element (`/Game/AktuelleTestregion(1VS1)/UIs/1vs1Spielfeld.PlayerBoxes` _1vs1spielfeld)
      (if (not (`/Game/AktuelleTestregion(1VS1)/UIs/KartenFeld.IsBelegt?` _array_element))
        (set `/Game/AktuelleTestregion(1VS1)/UIs/KartenFeld.CardPicture` "/Game/AktuelleTestregion(1VS1)/ImageFiles/Schwarz.Schwarz" _array_element)))
    (for _array_element_2 (`/Game/AktuelleTestregion(1VS1)/UIs/1vs1Spielfeld.PlayerFrontBoxes` _1vs1spielfeld)
      (if (not (`/Game/AktuelleTestregion(1VS1)/UIs/KartenFeld.IsBelegt?` _array_element_2))
        (set `/Game/AktuelleTestregion(1VS1)/UIs/KartenFeld.CardPicture` "/Game/AktuelleTestregion(1VS1)/ImageFiles/Schwarz.Schwarz" _array_element_2)))
    (for _array_element_3 (`/Game/AktuelleTestregion(1VS1)/UIs/1vs1Spielfeld.PlayerZauberplätze` _1vs1spielfeld)
      (if (not (`/Game/AktuelleTestregion(1VS1)/UIs/KartenFeld.IsBelegt?` _array_element_3))
        (set `/Game/AktuelleTestregion(1VS1)/UIs/KartenFeld.CardPicture` "/Game/AktuelleTestregion(1VS1)/ImageFiles/Schwarz.Schwarz" _array_element_3)))
    (for _array_element_4 (`/Game/AktuelleTestregion(1VS1)/UIs/1vs1Spielfeld.PlayersBuildingBoxes` _1vs1spielfeld)
      (if (not (`/Game/AktuelleTestregion(1VS1)/UIs/KartenFeld.IsBelegt?` _array_element_4))
        (set `/Game/AktuelleTestregion(1VS1)/UIs/KartenFeld.CardPicture` "/Game/AktuelleTestregion(1VS1)/ImageFiles/Schwarz.Schwarz" _array_element_4)))
    (else
      (for _array_element_5 (`/Game/AktuelleTestregion(1VS1)/UIs/1vs1Spielfeld.EnemyBoxes` _1vs1spielfeld)
        (if (not (`/Game/AktuelleTestregion(1VS1)/UIs/KartenFeld.IsBelegt?` _array_element_5))
          (set `/Game/AktuelleTestregion(1VS1)/UIs/KartenFeld.CardPicture` "/Game/AktuelleTestregion(1VS1)/ImageFiles/Schwarz.Schwarz" _array_element_5)))
      (for _array_element_6 (`/Game/AktuelleTestregion(1VS1)/UIs/1vs1Spielfeld.EnemyBuildingsBoxes` _1vs1spielfeld)
        (if (not (`/Game/AktuelleTestregion(1VS1)/UIs/KartenFeld.IsBelegt?` _array_element_6))
          (set `/Game/AktuelleTestregion(1VS1)/UIs/KartenFeld.CardPicture` "/Game/AktuelleTestregion(1VS1)/ImageFiles/Schwarz.Schwarz" _array_element_6)))
      (for _array_element_7 (`/Game/AktuelleTestregion(1VS1)/UIs/1vs1Spielfeld.EnemyFrontBoxes` _1vs1spielfeld)
        (if (not (`/Game/AktuelleTestregion(1VS1)/UIs/KartenFeld.IsBelegt?` _array_element_7))
          (set `/Game/AktuelleTestregion(1VS1)/UIs/KartenFeld.CardPicture` "/Game/AktuelleTestregion(1VS1)/ImageFiles/Schwarz.Schwarz" _array_element_7)))
      (for _array_element_8 (`/Game/AktuelleTestregion(1VS1)/UIs/1vs1Spielfeld.EnemyZauberplätze` _1vs1spielfeld)
        (if (not (`/Game/AktuelleTestregion(1VS1)/UIs/KartenFeld.IsBelegt?` _array_element_8))
          (set `/Game/AktuelleTestregion(1VS1)/UIs/KartenFeld.CardPicture` "/Game/AktuelleTestregion(1VS1)/ImageFiles/Schwarz.Schwarz" _array_element_7))))))

(fn `AlleBereit`
  (returns (Starten :type Boolean))
  (if (and (`self.Spieler1Bereit`) (`self.Spieler2Bereit`) (== (`KismetArrayLibrary.Array_Length` (`self.Spieler1Karten`)) 30) (== (`KismetArrayLibrary.Array_Length` (`self.Spieler2Karten`)) 30))
    (`/Game/Game/UI/Game/1VS1/Deckwählen.Bereit` (`self.DeckRef`))
    (set `self.Bereit` true)
    (else
      (set `self.Bereit` false)))
  (return (`self.Bereit`)))

(fn `DeckAusSpeicherLöschen`
  (params (NameDesDecks :type String))
  (bind (_gespeichertedecksspieler1 _gespeichertedecksspieler2) (break `/Game/AktuelleTestregion(1VS1)/Blueprints/DeckNamenSpeicher` (`self.DeckNamenSpeicherStructRef`)))
  (`GameplayStatics.DeleteGameInSlot` NameDesDecks)
  (setmembers `/Game/AktuelleTestregion(1VS1)/Blueprints/DeckNamenSpeicher` :`StructRef` (`self.DeckNamenSpeicherStructRef`) :`GespeicherteDecksSpieler1` _gespeichertedecksspieler1 :`GespeicherteDecksSpieler2` _gespeichertedecksspieler2))

(fn `GibKarten`
  (returns (Karten1 :type "Array of Integer") (Karten2 :type "Array of Integer"))
  (return (`self.Spieler1Karten`) (`self.Spieler2Karten`)))

(fn `GibNamen`
  (returns (Spieler1 :type String) (Spieler2 :type String))
  (return (`self.Name1`) (`self.Name2`)))

(fn `KarteAusgewählt`
  (returns (ZauberID :type Integer))
  (bind _aktuellezauberkartedieaufauswahlwartet (`self.AktuelleZauberKarteDieAufAuswahlWartet`))
  (`/Game/AktuelleTestregion(1VS1)/UIs/KartenFeld.AlleKArtenFreigeben` _aktuellezauberkartedieaufauswahlwartet)
  (return (`/Game/AktuelleTestregion(1VS1)/UIs/KartenFeld.EffektNummer` _aktuellezauberkartedieaufauswahlwartet)))

(fn `LadeSpeicher`
  (params (NameDesDecks :type String))
  (bind _returnvalue (`GameplayStatics.LoadGameFromSlot` NameDesDecks))
  (bind _asdeck_speicher (cast `/Game/AktuelleTestregion(1VS1)/Blueprints/DeckSpeicher` _returnvalue))
  (set `self.DeckSpeicherStructRef` (`/Game/AktuelleTestregion(1VS1)/Blueprints/DeckSpeicher.S DeckSpeicherAufbau` _asdeck_speicher)))

(fn `LadeSpeicherNamen`
  (returns (DecksSpieler1 :type "Array of String") (DecksSpieler2 :type "Array of String"))
  (bind _returnvalue (`GameplayStatics.LoadGameFromSlot` (`self.SpielerDecks`)))
  (bind _asdeck_speicher (cast `/Game/AktuelleTestregion(1VS1)/Blueprints/DeckSpeicher` _returnvalue))
  (bind _output_get (set `self.DeckNamenSpeicherStructRef` (`/Game/AktuelleTestregion(1VS1)/Blueprints/DeckSpeicher.S DeckNamenSpeicher` _asdeck_speicher)))
  (bind (_gespeichertedecksspieler1 _gespeichertedecksspieler2) (break `/Game/AktuelleTestregion(1VS1)/Blueprints/DeckNamenSpeicher` _output_get))
  (return _gespeichertedecksspieler1 _gespeichertedecksspieler2))

(fn `NeuenSpeicherOrtErstellen`)

(fn `Speichern`
  (params (NameDesDecks :type String))
  (bind _speicherref (`self.SpeicherRef`))
  (`/Engine/EditorBlueprintResources/StandardMacros.IsValid` (`self.SpeicherRef`)
    (:`Is Valid`
      _)
    (:`Is Not Valid`
      (bind _returnvalue (`GameplayStatics.CreateSaveGameObject` "/Game/AktuelleTestregion(1VS1)/Blueprints/DeckSpeicher.DeckSpeicher_C"))
      (set `self.SpeicherRef` _returnvalue)))
  (set `/Game/AktuelleTestregion(1VS1)/Blueprints/DeckSpeicher.S DeckSpeicherAufbau` (`self.DeckSpeicherStructRef`) _speicherref)
  (set `/Game/AktuelleTestregion(1VS1)/Blueprints/DeckSpeicher.S DeckNamenSpeicher` (`self.DeckNamenSpeicherStructRef`) _speicherref)
  (bind _returnvalue_2 (`GameplayStatics.SaveGameToSlot` (`self.SpeicherRef`) NameDesDecks))
  (if _returnvalue_2
    (`KismetSystemLibrary.PrintString` "Gespeichert!")
    (else
      (`KismetSystemLibrary.PrintString` "Fehler beim Speichern aufgetreten"))))

(fn `SpeichernDeckNamen`
  (`/Engine/EditorBlueprintResources/StandardMacros.IsValid` (`self.SpeicherRef`)
    (:`Is Valid`
      _)
    (:`Is Not Valid`
      (bind _returnvalue (`GameplayStatics.CreateSaveGameObject` "/Game/AktuelleTestregion(1VS1)/Blueprints/DeckSpeicher.DeckSpeicher_C"))
      (set `self.SpeicherRef` _returnvalue)))
  (set `/Game/AktuelleTestregion(1VS1)/Blueprints/DeckSpeicher.S DeckNamenSpeicher` (`self.DeckNamenSpeicherStructRef`) (`self.SpeicherRef`))
  (bind _returnvalue_2 (`GameplayStatics.SaveGameToSlot` (`self.SpeicherRef`) (`self.SpielerDecks`)))
  (if _returnvalue_2
    (`KismetSystemLibrary.PrintString` "Gespeichert!")
    (else
      (`KismetSystemLibrary.PrintString` "Fehler beim Speichern aufgetreten"))))

(fn `UserConstructionScript`)

(fn `ZähigkeitFunktion2`
  (returns (ZauberID :type Integer) (HP :type Integer) (DM :type Integer))
  (bind _aktuellezauberkartedieaufauswahlwartet (`self.AktuelleZauberKarteDieAufAuswahlWartet`))
  (bind _hpzaubermodifikator (`/Game/AktuelleTestregion(1VS1)/UIs/KartenFeld.HpZauberModifikator` _aktuellezauberkartedieaufauswahlwartet))
  (`/Game/AktuelleTestregion(1VS1)/UIs/KartenFeld.AlleKArtenFreigeben` _aktuellezauberkartedieaufauswahlwartet)
  (`KismetSystemLibrary.PrintString` (`KismetStringLibrary.Conv_IntToString` _hpzaubermodifikator))
  (return (`/Game/AktuelleTestregion(1VS1)/UIs/KartenFeld.EffektNummer` _aktuellezauberkartedieaufauswahlwartet) _hpzaubermodifikator (`/Game/AktuelleTestregion(1VS1)/UIs/KartenFeld.DmgZauberModifikator` _aktuellezauberkartedieaufauswahlwartet)))

(fn `ÜberprüfeSpeicherstand`
  (returns (`Existiert?` :type Boolean))
  (bind _returnvalue (`GameplayStatics.DoesSaveGameExist` (`self.SpielerDecks`)))
  (if _returnvalue
    (set `self.Existiert ein Deck im Speicher?` true)
    (else
      (set `self.Existiert ein Deck im Speicher?` false)))
  (return (`self.Existiert ein Deck im Speicher?`)))